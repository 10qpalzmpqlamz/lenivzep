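; Watchtower actor that teleports the player between two points and shows a UI widget while its trigger box is overlapped.
; Box overlap creates a Watchtower_wd widget and end overlap removes it, with no check on the overlapping actor.
; Telep moves the MPlayer character to Ex and TelepBack moves it to T1, both zeroing movement velocity afterward.
; Neither teleport event is called within this Blueprint.
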(event OnComponentBeginOverlap(Box)
  (params (OverlappedComponent :type Primitive%20Component%20Object%20Reference) (OtherActor :type Actor%20Object%20Reference) (OtherComp :type Primitive%20Component%20Object%20Reference) (OtherBodyIndex :type Integer) (bFromSweep :type Boolean) (SweepResult :type Hit%20Result%20Structure%20%28by%20ref%29))
  (bind _returnvalue (UserInterface|CreateWidget "/Game/watchtower_wd.watchtower_wd_C"))
  (UserInterface|Viewport|AddtoViewport _returnvalue 0))

(event OnComponentEndOverlap(Box)
  (params (OverlappedComponent :type Primitive%20Component%20Object%20Reference) (OtherActor :type Actor%20Object%20Reference) (OtherComp :type Primitive%20Component%20Object%20Reference) (OtherBodyIndex :type Integer))
  (Widget|RemovefromParent (stale OnComponentBeginOverlap(Box) _returnvalue)))

(event EventBeginPlay)

(event Collision|EventActorBeginOverlap
  (params (OtherActor :type Actor%20Object%20Reference)))

(event EventTick
  (params (DeltaSeconds :type Float%20%28single-precision%29)))

(event EventTelep
  (bind _returnvalue (Game|GetPlayerCharacter 0))
  (bind _ex (Variables|Default|Getex))
  (bind _returnvalue_2 (Transformation|GetWorldTransform _ex))
  (bind (_location _rotation) (Math|Transform|BreakTransform _returnvalue_2))
  (bind _asmplayer (Utilities|Casting|CastToMPlayer _returnvalue))
  (Transformation|Teleport _asmplayer _location _rotation)
  (Variables|/Script/Engine.MovementComponent|SetVelocity (Variables|/Script/Engine.Character|GetCharacterMovement _returnvalue) "0, 0, 0"))

(event EventTelepBack
  (bind _returnvalue (Game|GetPlayerCharacter 0))
  (bind _t1 (Variables|Default|Gett1))
  (bind _returnvalue_2 (Transformation|GetWorldTransform _t1))
  (bind (_location _rotation) (Math|Transform|BreakTransform _returnvalue_2))
  (bind _asmplayer (Utilities|Casting|CastToMPlayer _returnvalue))
  (Transformation|Teleport _asmplayer _location _rotation)
  (Variables|/Script/Engine.MovementComponent|SetVelocity (Variables|/Script/Engine.Character|GetCharacterMovement _returnvalue) "0, 0, 0"))

(fn ConstructionScript)